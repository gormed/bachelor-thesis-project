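; Base drinkable item that drains its liquid into a BP_CaedeCharacter's drinking, poison, urine and alcohol levels.
; Construction derives per-unit effect rates, which TickDrink scales by flow and delta time, with urine transfer gated on the Poison value.
; Start and end calls toggle the character's drinking flags by stance.
; Weight shrinks with the remaining amount, and an emptied drink is marked consumed and dropped.
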(event `self.ReceiveBeginPlay`)

(fn `ActualWeight`
  (returns (ReturnValue :type "Float (double-precision)"))
  (bind _emptyweight (`self.EmptyWeight`))
  (return (+ (* (/ (`self.Amount`) (`self.StartAmount`)) (- (`self.FullWeight`) _emptyweight)) _emptyweight)))

(fn `Disable Drink Mode`
  (params (character :type "CaedeCharacter Object Reference (by ref)"))
  (bind _asbp_caede_character (cast `/Game/Blueprints/MainCharacter/BP_CaedeCharacter` character))
  (set `/Game/Blueprints/MainCharacter/BP_CaedeCharacter.IsDrinkingOneHand?` false _asbp_caede_character)
  (set `/Game/Blueprints/MainCharacter/BP_CaedeCharacter.IsDrinkingTwoHand?` false _asbp_caede_character)
  (set `/Game/Blueprints/MainCharacter/BP_CaedeCharacter.IsDrinkingFriendly?` false _asbp_caede_character)
  (set `/Game/Blueprints/MainCharacter/BP_CaedeCharacter.IsDrinkingBow?` false _asbp_caede_character))

(fn `Enable Drink Mode`
  (params (character :type "CaedeCharacter Object Reference (by ref)"))
  (bind _asbp_caede_character (cast `/Game/Blueprints/MainCharacter/BP_CaedeCharacter` character))
  (if (`/Game/Blueprints/MainCharacter/BP_CaedeCharacter.IsHoldingOneHand?` _asbp_caede_character)
    (set `/Game/Blueprints/MainCharacter/BP_CaedeCharacter.IsDrinkingOneHand?` true _asbp_caede_character))
  (if (`/Game/Blueprints/MainCharacter/BP_CaedeCharacter.IsHoldingTwoHand?` _asbp_caede_character)
    (set `/Game/Blueprints/MainCharacter/BP_CaedeCharacter.IsDrinkingTwoHand?` true _asbp_caede_character))
  (if (`/Game/Blueprints/MainCharacter/BP_CaedeCharacter.IsFriendlyMode?` _asbp_caede_character)
    (set `/Game/Blueprints/MainCharacter/BP_CaedeCharacter.IsDrinkingFriendly?` true _asbp_caede_character))
  (if (`/Game/Blueprints/MainCharacter/BP_CaedeCharacter.IsInBowMode?` _asbp_caede_character)
    (set `/Game/Blueprints/MainCharacter/BP_CaedeCharacter.IsDrinkingBow?` true _asbp_caede_character)))

(fn `EndDrink`
  (params (character :type "CaedeCharacter Object Reference"))
  (bind _asbp_caede_character (cast `/Game/Blueprints/MainCharacter/BP_CaedeCharacter` character))
  (if (not (`self.IsConsumed`))
    (`self.Disable Drink Mode` _asbp_caede_character)))

(fn `IsEmpty`
  (returns (ReturnValue :type Boolean))
  (return (<= (`self.Amount`) 0.0)))

(fn `PercentageAmount`
  (returns (ReturnValue :type "Float (double-precision)"))
  (return (/ (`self.Amount`) (`self.StartAmount`))))

(fn `StartDrink`
  (params (Character :type "CaedeCharacter Object Reference"))
  (bind _asbp_caede_character (cast `/Game/Blueprints/MainCharacter/BP_CaedeCharacter` Character))
  (if (not (`self.IsConsumed`))
    (`self.Enable Drink Mode` _asbp_caede_character)))

(fn `TickDrink`
  (params (Character :type "CaedeCharacter Object Reference") (DeltaTime :type "Float (double-precision)"))
  (bind _amount (`self.Amount`))
  (bind _urinticked (`self.UrinTicked`))
  (bind _poison (`self.Poison`))
  (bind _poison_2 (`self.Poison`))
  (bind _alcohol (`self.Alcohol`))
  (bind _returnvalue (* DeltaTime (`self.FlowAmount`)))
  (bind _returnvalue_2 (* _returnvalue (`self.PoisonTicked`)))
  (bind _returnvalue_3 (* _returnvalue (`self.AlcoholTicked`)))
  (bind _asbp_caede_character (cast `/Game/Blueprints/MainCharacter/BP_CaedeCharacter` Character))
  ;[1 1 1] Regenerate Drinking
  (if (not (`self.IsConsumed`))
    (if (> _amount 0.0)
      (set `self.Amount` (- _amount _returnvalue))
      (set `/Game/Blueprints/MainCharacter/BP_CaedeCharacter.Drinking` (`KismetMathLibrary.FClamp` (+ _returnvalue (`/Game/Blueprints/MainCharacter/BP_CaedeCharacter.Drinking` _asbp_caede_character)) 0.0 100.0) _asbp_caede_character)
      ;[1 1 1] Set Poison Value
      (if (> _poison 0.0)
        (set `self.Poison` (- _poison _returnvalue_2))
        (set `/Game/Blueprints/MainCharacter/BP_CaedeCharacter.Poison` (`KismetMathLibrary.FClamp` (+ _returnvalue_2 (`/Game/Blueprints/MainCharacter/BP_CaedeCharacter.Poison` _asbp_caede_character)) 0.0 100.0) _asbp_caede_character))
      ;[1 1 1] Urin Level
      (if (> _poison_2 0.0)
        (set `self.Urin` (- _poison_2 _urinticked))
        (set `/Game/Blueprints/MainCharacter/BP_CaedeCharacter.UrinLevel` (`KismetMathLibrary.FClamp` (+ (* _returnvalue _urinticked) (`/Game/Blueprints/MainCharacter/BP_CaedeCharacter.UrinLevel` _asbp_caede_character)) 0.0 100.0) _asbp_caede_character))
      ;[1 1 1] Alcohol Level
      (if (> _alcohol 0.0)
        (set `self.Alcohol` (- _alcohol _returnvalue_3))
        (set `/Game/Blueprints/MainCharacter/BP_CaedeCharacter.AlcoholLevel` (`KismetMathLibrary.FClamp` (+ _returnvalue_3 (`/Game/Blueprints/MainCharacter/BP_CaedeCharacter.AlcoholLevel` _asbp_caede_character)) 0.0 100.0) _asbp_caede_character))
      (bind _returnvalue_4 (`self.ActualWeight`))
      (`self.ChangeWeight` _returnvalue_4)
      (else
        (set `self.IsConsumed` true)
        (`self.Disable Drink Mode` _asbp_caede_character)
        (`self.DropItem` _asbp_caede_character)))))

(fn `UserConstructionScript`
  (bind _amount (`self.Amount`))
  (`parent.UserConstructionScript`)
  (set `self.PoisonTicked` (/ (`self.Poison`) _amount))
  (set `self.UrinTicked` (/ (`self.Urin`) _amount))
  (set `self.AlcoholTicked` (/ (`self.Alcohol`) _amount))
  (set `self.StartAmount` _amount))