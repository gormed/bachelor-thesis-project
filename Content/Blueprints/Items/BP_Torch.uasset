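; BP_Torch is a holdable torch item that shows or hides its flame particles and point light through ToggleTorchLight.
; The construction script and BeginPlay set the initial state from IsBurning, then BeginPlay binds the grab and selection events.
; Grabbing briefly raises the BP_CaedeCharacter's one-hand pickup flag, then lights the torch after the delay.
; Selecting or unselecting shows or hides both actor and light, without updating IsBurning.
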(event `self.ReceiveBeginPlay`
  (`|ExecutionSequence`
    (:`then_0`
      (`self.ToggleTorchLight` (`self.IsBurning`)))
    (:`then_1`
      ;[1 1 1] Pickup
      (add `self.OnStartItemGrab` (delegate `OnStartItemGrab_Event`))
      (add `self.OnEndItemGrab` (delegate `OnEndItemGrab_Event`))
      ;[1 1 1] Unselect Weapon
      (add `self.OnIsUnselected` (delegate `OnIsUnselected_Event`))
      ;[1 1 1] Select Weapon
      (add `self.OnIsSelected` (delegate `OnIsSelected_Event`)))))

(event `OnStartItemGrab_Event` :!signature `self.OnStartItemGrab`
  (params (InteractsWith :type "CaedeCharacter Object Reference"))
  ;[1 1 1] Pickup
  (bind _asbp_caede_character (cast `/Game/Blueprints/MainCharacter/BP_CaedeCharacter` InteractsWith))
  (set `/Game/Blueprints/MainCharacter/BP_CaedeCharacter.IsPickup_OneHand_Weapon?` true _asbp_caede_character)
  (`KismetSystemLibrary.Delay` 1.7)
  (set `/Game/Blueprints/MainCharacter/BP_CaedeCharacter.IsPickup_OneHand_Weapon?` false _asbp_caede_character)
  (`self.ToggleTorchLight` true))

(event `OnEndItemGrab_Event` :!signature `self.OnEndItemGrab`
  (params (InteractsWith :type "CaedeCharacter Object Reference")))

(event `OnIsUnselected_Event` :!signature `self.OnIsUnselected`
  (params (SelectedBy :type "CaedeCharacter Object Reference") (handSlot :type "InteractionComponent.EHandSlot Enum"))
  ;[1 1 1] Unselect Weapon
  (cast `/Game/Blueprints/MainCharacter/BP_CaedeCharacter` SelectedBy)
  (`self.SetActorHiddenInGame` true)
  (`self.ToggleTorchLight` false))

(event `OnIsSelected_Event` :!signature `self.OnIsSelected`
  (params (SelectedBy :type "CaedeCharacter Object Reference") (handSlot :type "InteractionComponent.EHandSlot Enum"))
  ;[1 1 1] Select Weapon
  (cast `/Game/Blueprints/MainCharacter/BP_CaedeCharacter` SelectedBy)
  (`self.SetActorHiddenInGame` false)
  (`self.ToggleTorchLight` true))

(fn `ToggleTorchLight`
  (params (Enable :type Boolean))
  (`SceneComponent.SetVisibility` (`self.ParticleSystem1`) Enable false)
  (`SceneComponent.SetVisibility` (`self.PointLight1`) Enable false))

(fn `UserConstructionScript`
  (`self.ToggleTorchLight` (`self.IsBurning`)))