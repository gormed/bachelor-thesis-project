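; BP_DrugItem is a consumable drug item that raises a BP_CaedeCharacter's DrugLevel gradually as it is drunk.
; StartDrug and EndDrug toggle the character's drinking flags, with EnableDrugMode choosing them from the current hold, friendly or bow mode.
; TickDrug drains Amount at FlowAmount into the clamped drug level and scales item weight from full toward empty.
; Once Amount runs out, the item is marked consumed, drinking stops and it is dropped.
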(fn `ActualWeight`
  (returns (ReturnValue :type "Float (double-precision)"))
  (bind _emptyweight (`self.EmptyWeight`))
  (return (+ (* (/ (`self.Amount`) (`self.StartAmount`)) (- (`self.FullWeight`) _emptyweight)) _emptyweight)))

(fn `DisableDrugMode`
  (params (Character :type "Character Object Reference"))
  (bind _asbp_caede_character (cast `/Game/Blueprints/MainCharacter/BP_CaedeCharacter` Character))
  (set `/Game/Blueprints/MainCharacter/BP_CaedeCharacter.IsDrinkingOneHand?` false _asbp_caede_character)
  (set `/Game/Blueprints/MainCharacter/BP_CaedeCharacter.IsDrinkingTwoHand?` false _asbp_caede_character)
  (set `/Game/Blueprints/MainCharacter/BP_CaedeCharacter.IsDrinkingFriendly?` false _asbp_caede_character)
  (set `/Game/Blueprints/MainCharacter/BP_CaedeCharacter.IsDrinkingBow?` false _asbp_caede_character))

(fn `EnableDrugMode`
  (params (Character :type "Character Object Reference"))
  (bind _asbp_caede_character (cast `/Game/Blueprints/MainCharacter/BP_CaedeCharacter` Character))
  (if (`/Game/Blueprints/MainCharacter/BP_CaedeCharacter.IsHoldingOneHand?` _asbp_caede_character)
    (set `/Game/Blueprints/MainCharacter/BP_CaedeCharacter.IsDrinkingOneHand?` true _asbp_caede_character))
  (if (`/Game/Blueprints/MainCharacter/BP_CaedeCharacter.IsHoldingTwoHand?` _asbp_caede_character)
    (set `/Game/Blueprints/MainCharacter/BP_CaedeCharacter.IsDrinkingTwoHand?` true _asbp_caede_character))
  (if (`/Game/Blueprints/MainCharacter/BP_CaedeCharacter.IsFriendlyMode?` _asbp_caede_character)
    (set `/Game/Blueprints/MainCharacter/BP_CaedeCharacter.IsDrinkingFriendly?` true _asbp_caede_character))
  (if (`/Game/Blueprints/MainCharacter/BP_CaedeCharacter.IsInBowMode?` _asbp_caede_character)
    (set `/Game/Blueprints/MainCharacter/BP_CaedeCharacter.IsDrinkingBow?` true _asbp_caede_character)))

(fn `EndDrug`
  (params (Character :type "Character Object Reference"))
  (bind _asbp_caede_character (cast `/Game/Blueprints/MainCharacter/BP_CaedeCharacter` Character))
  (if (not (`self.IsConsumed`))
    (`self.DisableDrugMode` _asbp_caede_character)))

(fn `IsEmpty`
  (returns (ReturnValue :type Boolean))
  (return (<= (`self.Amount`) 0.0)))

(fn `StartDrug`
  (params (Character :type "Character Object Reference"))
  (bind _asbp_caede_character (cast `/Game/Blueprints/MainCharacter/BP_CaedeCharacter` Character))
  (if (not (`self.IsConsumed`))
    (`self.EnableDrugMode` _asbp_caede_character)))

(fn `TickDrug`
  (params (Character :type "Character Object Reference") (DeltaTime :type "Float (double-precision)"))
  (bind _returnvalue (* DeltaTime (`self.FlowAmount`)))
  (bind _asbp_caede_character (cast `/Game/Blueprints/MainCharacter/BP_CaedeCharacter` Character))
  (if (and (> (`self.Amount`) 0.0) (not (`self.IsConsumed`)))
    ;[1 1 1] Drug Level
    (set `self.Amount` (- (`self.Amount`) _returnvalue))
    (set `/Game/Blueprints/MainCharacter/BP_CaedeCharacter.DrugLevel` (`KismetMathLibrary.FClamp` (+ _returnvalue (`/Game/Blueprints/MainCharacter/BP_CaedeCharacter.DrugLevel` _asbp_caede_character)) 0.0 100.0) _asbp_caede_character)
    (bind _returnvalue_2 (`self.ActualWeight`))
    (`self.ChangeWeight` _returnvalue_2)
    (else
      (set `self.IsConsumed` true)
      (`self.DisableDrugMode` _asbp_caede_character)
      (`self.DropItem` _asbp_caede_character))))

(fn `UserConstructionScript`
  (bind _amount (`self.Amount`))
  (`parent.UserConstructionScript`)
  (set `self.DrugTicked` (/ (`self.Drug`) _amount))
  (set `self.StartAmount` _amount))