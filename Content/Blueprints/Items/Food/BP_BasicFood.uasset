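; Base food item that a BP_CaedeCharacter consumes gradually while using it, altering stats such as health, stamina, poison and alcohol.
; Construction precomputes per-unit effects; item-use start and end events toggle the character's drinking pose flags.
; Each use tick drains Amount, feeds clamped stats and updates weight, then drops the item once empty.
; The urine effect is gated on Poison, and the Shit transfer multiplies by zero.
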(event `self.ReceiveBeginPlay`
  (add `self.OnStartItemUse` (delegate `OnStartItemUse_Event_Copy`))
  (add `self.OnEndItemUse` (delegate `OnEndItemUse_Event_Copy`))
  (add `self.OnTickItemUse` (delegate `OnTickItemUse_Event_Copy`)))

(event `OnStartItemUse_Event_Copy` :!signature `self.OnStartItemUse`
  (params (UsedBy :type "CaedeCharacter Object Reference"))
  (`self.StartEat` UsedBy))

(event `OnEndItemUse_Event_Copy` :!signature `self.OnEndItemUse`
  (params (UsedBy :type "CaedeCharacter Object Reference"))
  (`self.EndEat` UsedBy))

(event `OnTickItemUse_Event_Copy` :!signature `self.OnTickItemUse`
  (params (DeltaTime :type "Float (double-precision)") (UsedBy :type "CaedeCharacter Object Reference"))
  (`self.TickEat` UsedBy DeltaTime))

(fn `ActualWeight`
  (returns (ReturnValue :type "Float (double-precision)"))
  (bind _emptyweight (`self.EmptyWeight`))
  (return (+ (* (/ (`self.Amount`) (`self.StartAmount`)) (- (`self.FullWeight`) _emptyweight)) _emptyweight)))

(fn `Disable Eat Mode`
  (params (character :type "CaedeCharacter Object Reference (by ref)"))
  (bind _asbp_caede_character (cast `/Game/Blueprints/MainCharacter/BP_CaedeCharacter` character))
  (set `/Game/Blueprints/MainCharacter/BP_CaedeCharacter.IsDrinkingOneHand?` false _asbp_caede_character)
  (set `/Game/Blueprints/MainCharacter/BP_CaedeCharacter.IsDrinkingTwoHand?` false _asbp_caede_character)
  (set `/Game/Blueprints/MainCharacter/BP_CaedeCharacter.IsDrinkingFriendly?` false _asbp_caede_character)
  (set `/Game/Blueprints/MainCharacter/BP_CaedeCharacter.IsDrinkingBow?` false _asbp_caede_character))

(fn `Enable Eat Mode`
  (params (character :type "CaedeCharacter Object Reference (by ref)"))
  (bind _asbp_caede_character (cast `/Game/Blueprints/MainCharacter/BP_CaedeCharacter` character))
  (if (`/Game/Blueprints/MainCharacter/BP_CaedeCharacter.IsHoldingOneHand?` _asbp_caede_character)
    (set `/Game/Blueprints/MainCharacter/BP_CaedeCharacter.IsDrinkingOneHand?` true _asbp_caede_character))
  (if (`/Game/Blueprints/MainCharacter/BP_CaedeCharacter.IsHoldingTwoHand?` _asbp_caede_character)
    (set `/Game/Blueprints/MainCharacter/BP_CaedeCharacter.IsDrinkingTwoHand?` true _asbp_caede_character))
  (if (`/Game/Blueprints/MainCharacter/BP_CaedeCharacter.IsFriendlyMode?` _asbp_caede_character)
    (set `/Game/Blueprints/MainCharacter/BP_CaedeCharacter.IsDrinkingFriendly?` true _asbp_caede_character))
  (if (`/Game/Blueprints/MainCharacter/BP_CaedeCharacter.IsInBowMode?` _asbp_caede_character)
    (set `/Game/Blueprints/MainCharacter/BP_CaedeCharacter.IsDrinkingBow?` true _asbp_caede_character)))

(fn `EndEat`
  (params (character :type "CaedeCharacter Object Reference (by ref)"))
  (bind _asbp_caede_character (cast `/Game/Blueprints/MainCharacter/BP_CaedeCharacter` character))
  (if (not (`self.IsConsumed`))
    (`self.Disable Eat Mode` _asbp_caede_character)))

(fn `IsEmpty`
  (returns (ReturnValue :type Boolean))
  (return (<= (`self.Amount`) 0.0)))

(fn `PercentageAmount`
  (returns (ReturnValue :type "Float (double-precision)"))
  (return (/ (`self.Amount`) (`self.StartAmount`))))

(fn `StartEat`
  (params (character :type "CaedeCharacter Object Reference (by ref)"))
  (bind _asbp_caede_character (cast `/Game/Blueprints/MainCharacter/BP_CaedeCharacter` character))
  (if (not (`self.IsConsumed`))
    (`self.Enable Eat Mode` _asbp_caede_character)))

(fn `TickEat`
  (params (character :type "CaedeCharacter Object Reference (by ref)") (DeltaTiime :type "Float (double-precision)"))
  (bind _amount (`self.Amount`))
  (bind _urinticked (`self.UrinTicked`))
  (bind _poison (`self.Poison`))
  (bind _alcohol (`self.Alcohol`))
  (bind _stamina (`self.Stamina`))
  (bind _shit (`self.Shit`))
  (bind _health (`self.Health`))
  (bind _poison_2 (`self.Poison`))
  (bind _returnvalue (* DeltaTiime (`self.FlowAmount`)))
  (bind _returnvalue_2 (* 0.0 (`self.ShitTicked`)))
  (bind _returnvalue_3 (* _returnvalue (`self.PoisonTicked`)))
  (bind _returnvalue_4 (* _returnvalue (`self.AlcoholTicked`)))
  (bind _returnvalue_5 (* _returnvalue (`self.StaminaTicked`)))
  (bind _returnvalue_6 (* _returnvalue (`self.HealthTicked`)))
  (if (not (`self.IsConsumed`))
    (bind _asbp_caede_character (cast `/Game/Blueprints/MainCharacter/BP_CaedeCharacter` character))
    ;[1 1 1] Eating
    (if (> _amount 0.0)
      (set `self.Amount` (- _amount _returnvalue))
      (set `/Game/Blueprints/MainCharacter/BP_CaedeCharacter.Eating` (`KismetMathLibrary.FClamp` (+ _returnvalue (`/Game/Blueprints/MainCharacter/BP_CaedeCharacter.Eating` _asbp_caede_character)) 0.0 100.0) _asbp_caede_character)
      ;[1 1 1] Health
      (if (> _health 0.0)
        (set `self.Health` (- _health _returnvalue_6))
        (set `/Game/Blueprints/MainCharacter/BP_CaedeCharacter.Health` (`KismetMathLibrary.FClamp` (+ _returnvalue_6 (`/Game/Blueprints/MainCharacter/BP_CaedeCharacter.Health` _asbp_caede_character)) 0.0 100.0) _asbp_caede_character))
      ;[1 1 1] Poison
      (if (> _poison 0.0)
        (set `self.Poison` (- _poison _returnvalue_3))
        (set `/Game/Blueprints/MainCharacter/BP_CaedeCharacter.Poison` (`KismetMathLibrary.FClamp` (+ _returnvalue_3 (`/Game/Blueprints/MainCharacter/BP_CaedeCharacter.Poison` _asbp_caede_character)) 0.0 100.0) _asbp_caede_character))
      ;[1 1 1] Urin
      (if (> _poison_2 0.0)
        (set `self.Urin` (- _poison_2 _urinticked))
        (set `/Game/Blueprints/MainCharacter/BP_CaedeCharacter.UrinLevel` (`KismetMathLibrary.FClamp` (+ (* _returnvalue _urinticked) (`/Game/Blueprints/MainCharacter/BP_CaedeCharacter.UrinLevel` _asbp_caede_character)) 0.0 100.0) _asbp_caede_character))
      ;[1 1 1] Alcohol
      (if (> _alcohol 0.0)
        (set `self.Alcohol` (- _alcohol _returnvalue_4))
        (set `/Game/Blueprints/MainCharacter/BP_CaedeCharacter.AlcoholLevel` (`KismetMathLibrary.FClamp` (+ _returnvalue_4 (`/Game/Blueprints/MainCharacter/BP_CaedeCharacter.AlcoholLevel` _asbp_caede_character)) 0.0 100.0) _asbp_caede_character))
      ;[1 1 1] Stamina
      (if (> _stamina 0.0)
        (set `self.Stamina` (- _stamina _returnvalue_5))
        (set `/Game/Blueprints/MainCharacter/BP_CaedeCharacter.Stamina` (`KismetMathLibrary.FClamp` (+ _returnvalue_5 (`/Game/Blueprints/MainCharacter/BP_CaedeCharacter.Stamina` _asbp_caede_character)) 0.0 100.0) _asbp_caede_character))
      ;[1 1 1] Shit
      (if (> _shit 0.0)
        (set `self.Shit` (- _shit _returnvalue_2))
        (set `/Game/Blueprints/MainCharacter/BP_CaedeCharacter.ShitLevel` (`KismetMathLibrary.FClamp` (+ _returnvalue_2 (`/Game/Blueprints/MainCharacter/BP_CaedeCharacter.ShitLevel` _asbp_caede_character)) 0.0 100.0) _asbp_caede_character))
      (bind _returnvalue_7 (`self.ActualWeight`))
      (`self.ChangeWeight` _returnvalue_7)
      (else
        (set `self.IsConsumed` true)
        (`self.Disable Eat Mode` _asbp_caede_character)
        (`self.DropItem` _asbp_caede_character)))))

(fn `UserConstructionScript`
  (bind _amount (`self.Amount`))
  (`parent.UserConstructionScript`)
  (set `self.PoisonTicked` (/ (`self.Poison`) _amount))
  (set `self.UrinTicked` (/ (`self.Urin`) _amount))
  (set `self.AlcoholTicked` (/ (`self.Alcohol`) _amount))
  (set `self.HealthTicked` (/ (`self.Health`) _amount))
  (set `self.ShitTicked` (/ (`self.Shit`) _amount))
  (set `self.StaminaTicked` (/ (`self.Stamina`) _amount))
  (set `self.StartAmount` _amount))