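; Item spawner actor that spawns random picks from SpawnItems within a sphere, capsule or box, at spawn points, or at its own location.
; Tick fires the OnItemSpawn dispatcher at a world time or on a repeating duration timer, and toggles debug visibility.
; The bound event spawns batches with random delays and optional random rotation and scale, recording spawned actors.
; The construction script filters out non-Item classes and configures the selected shape's preview.
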(event `self.ReceiveBeginPlay`
  (add `self.OnItemSpawn` (delegate `OnItemSpawn_Event`)))

(event `OnItemSpawn_Event` :!signature `self.OnItemSpawn`
  (params (WorldTime :type "WorldTime Object Reference"))
  ;[1 1 1] Trigger Spawning
  (if (`self.StartsDelayed`)
    (`KismetSystemLibrary.Delay` (`self.StartDelay`)))
  (for _ (range (`self.ItemSpawnCount`))
    (`self.DoSpawnRandom`)
    (`KismetSystemLibrary.Delay` (`KismetMathLibrary.RandomFloatInRange` (`self.ItemSpawnMinDelay`) (`self.ItemSpawnMaxDelay`)))))

(event `self.ReceiveTick`
  (params (DeltaSeconds :type "Float (single-precision)"))
  (bind _repeatcounter (`self.RepeatCounter`))
  (bind _repeat_times (`self.Repeat Times`))
  (bind _repeatcounter_2 (`self.RepeatCounter`))
  (bind _repeat_times_2 (`self.Repeat Times`))
  (bind _returnvalue (not (`self.Draw Debug`)))
  (set `self.DeltaTime` DeltaSeconds)
  ;[1 1 1] Debug
  (for _array_element (`self.SpawnPoints`)
    (`self.SetActorHiddenInGame` _array_element _returnvalue)
    (`SceneComponent.SetHiddenInGame` (`TargetPoint.SpriteComponent` _array_element) _returnvalue _returnvalue))
  (`SceneComponent.SetHiddenInGame` (`self.Sphere`) _returnvalue _returnvalue)
  (`SceneComponent.SetHiddenInGame` (`self.Capsule`) _returnvalue _returnvalue)
  (`SceneComponent.SetHiddenInGame` (`self.Box`) _returnvalue _returnvalue)
  (if (`self.Fixed Time`)
    ;[1 1 1] Time
    (bind _returnvalue_2 (`WorldTime.Get2400Format` (`self.World Time`)))
    (if (and (> _returnvalue_2 (`self.Spawn Time`)) (xor (< _repeatcounter_2 _repeat_times_2) (< _repeat_times_2 0)))
      (set `self.RepeatCounter` (+ _repeatcounter_2 1))
      (`self.TriggerSpawn` (`self.World Time`)))
    (elif (`self.FixedDuration`)
      ;[1 1 1] Duration
      (set `self.DurationTimer` (+ (`self.DurationTimer`) (`self.DeltaTime`)))
      (if (and (>= (`self.DurationTimer`) (`self.Duration`)) (xor (< _repeatcounter _repeat_times) (< _repeat_times 0)))
        (set `self.DurationTimer` 0.0)
        (set `self.RepeatCounter` (+ _repeatcounter 1))
        (`self.TriggerSpawn` (`self.World Time`))))))

(fn `DoSpawnRandom`
  (bind _spawnitems (`self.SpawnItems`))
  (bind _spawnpoints (`self.SpawnPoints`))
  ;[0 1 0.3995 0.257] Spawn
  (bind _asactor (castclass `Actor` (`KismetArrayLibrary.Array_Get` _spawnitems (`KismetMathLibrary.RandomIntegerInRange` 0 (- (`KismetArrayLibrary.Array_Length` _spawnitems) 1))))
    (:`then`
      (if (`self.RandomRotation`)
        (set `self.RandomRot` (`KismetMathLibrary.RandomRotator` true)))
      (if (`self.RandomScale`)
        (set `self.RadomScale` (* (`KismetMathLibrary.RandomUnitVector`) (`KismetMathLibrary.RandomFloatInRange` (`self.MinScale`) (`self.MaxScale`)))))
      (if (`self.RandomLocation`)
        (switch `/Game/Blueprints/Items/E_ItemSpawnShape` (`self.SpawnShape`)
          (:`NewEnumerator0`
            (set `self.SpawnTransform` (`KismetMathLibrary.MakeTransform` (+ (* (`KismetMathLibrary.RandomUnitVector`) (`self.Radius`)) (`self.K2_GetActorLocation`)) (`self.RandomRot`) (`self.RadomScale`))))
          (:`NewEnumerator1`
            (set `self.SpawnTransform` (`KismetMathLibrary.MakeTransform` (+ (`KismetMathLibrary.MakeVector` (.x (* (`KismetMathLibrary.RandomUnitVector`) (`self.Radius`))) (.y (* (`KismetMathLibrary.RandomUnitVector`) (`self.Radius`))) (+ (.z (* (`KismetMathLibrary.RandomUnitVector`) (`self.Radius`))) (`KismetMathLibrary.RandomFloatInRange` 0.0 (`self.Height`)))) (`self.K2_GetActorLocation`)) (`self.RandomRot`) (`self.RadomScale`))))
          (:`NewEnumerator2`
            (set `self.SpawnTransform` (`KismetMathLibrary.MakeTransform` (+ (`KismetMathLibrary.MakeVector` (`KismetMathLibrary.RandomFloatInRange` 0.0 (.x (`self.Box Size`))) (`KismetMathLibrary.RandomFloatInRange` 0.0 (.y (`self.Box Size`))) (`KismetMathLibrary.RandomFloatInRange` 0.0 (.z (`self.Box Size`)))) (`self.K2_GetActorLocation`)) (`self.RandomRot`) (`self.RadomScale`))))
          (:`NewEnumerator4`
            (set `self.SpawnTransform` (`KismetMathLibrary.MakeTransform` (`self.K2_GetActorLocation` (`KismetArrayLibrary.Array_Get` _spawnpoints (`KismetMathLibrary.RandomIntegerInRange` 0 (- (`KismetArrayLibrary.Array_Length` _spawnpoints) 1)))) (`self.RandomRot`) (`self.RadomScale`)))))
        (else
          (set `self.SpawnTransform` (`KismetMathLibrary.MakeTransform` (`self.K2_GetActorLocation`) (`self.RandomRot`) (`self.RadomScale`)))))
      (bind _returnvalue (`|SpawnActorFromClass` _asactor (`self.SpawnTransform`) (`self.Force Spawn`)))
      (`KismetArrayLibrary.Array_Add` (`self.SpawnedActors`) _returnvalue))
    (:`CastFailed`
      _))
  (return))

(fn `TriggerSpawn`
  (params (WorldTime :type "WorldTime Object Reference"))
  (`self.OnItemSpawn` WorldTime))

(fn `UserConstructionScript`
  (bind _capsule (`self.Capsule`))
  (bind _box (`self.Box`))
  (bind _sphere (`self.Sphere`))
  (bind _points (`self.Points`))
  (`SceneComponent.SetRelativeLocation` (`self.Offset`) (`self.Position Offset`) true)
  ;[1 0.2106 0 0.577] Check For Item Base Class
  (`KismetArrayLibrary.Array_Clear` (`self.InvalidSpawnItems`))
  (for _array_element (`self.SpawnItems`)
    (if (not (xor (== _array_element null) (`KismetMathLibrary.ClassIsChildOf` _array_element "/Script/Caede.Item")))
      (`KismetArrayLibrary.Array_Add` (`self.InvalidSpawnItems`) _array_element)))
  (for _array_element_2 (`self.InvalidSpawnItems`)
    (`KismetArrayLibrary.Array_RemoveItem` (`self.SpawnItems`) _array_element_2))
  ;[1 1 1] Switch Between Mode
  (switch `/Game/Blueprints/Items/E_ItemSpawnShape` (`self.SpawnShape`)
    (:`NewEnumerator0`
      (`SceneComponent.SetVisibility` _points false true)
      (`SceneComponent.SetVisibility` _capsule false true)
      (`SceneComponent.SetVisibility` _box false true)
      (`SceneComponent.SetVisibility` _sphere true true)
      (`SphereComponent.SetSphereRadius` _sphere (`self.Radius`) true))
    (:`NewEnumerator1`
      (`SceneComponent.SetVisibility` _points true true)
      (`SceneComponent.SetVisibility` _capsule true true)
      (`SceneComponent.SetVisibility` _box false true)
      (`SceneComponent.SetVisibility` _sphere false true)
      (`CapsuleComponent.SetCapsuleHalfHeight` _capsule (`self.Height`) true)
      (`CapsuleComponent.SetCapsuleRadius` _capsule (`self.Radius`) true))
    (:`NewEnumerator2`
      (`SceneComponent.SetVisibility` _points false true)
      (`SceneComponent.SetVisibility` _capsule false true)
      (`SceneComponent.SetVisibility` _box true true)
      (`SceneComponent.SetVisibility` _sphere false true)
      (`BoxComponent.SetBoxExtent` _box (`self.Box Size`) true))
    (:`NewEnumerator4`
      (`SceneComponent.SetVisibility` _points true true)
      (`SceneComponent.SetVisibility` _capsule false true)
      (`SceneComponent.SetVisibility` _box false true)
      (`SceneComponent.SetVisibility` _sphere false true)
      (for _array_element_3 (`self.SpawnPoints`)
        (`/Engine/EditorBlueprintResources/StandardMacros.IsValid` _array_element_3
          (:`Is Valid`
            (`self.AttachRootComponentTo` _array_element_3 (`self.Points`) "None" "KeepWorldPosition")))))))