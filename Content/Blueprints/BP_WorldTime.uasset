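; World time Blueprint that switches post-process volumes between day and night settings based on the current clock time.
; Each Tick, UpdatePostProcessingVolumes compares 24-hour time to day start and end, copies the matching settings, and interpolates ambient cubemap intensity.
; TrueSky time setting and sun, moon and ambient light updates are disconnected in both Tick and the Construction Script, as is the instant construction-time volume update.
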(event `self.ReceiveTick`
  (params (DeltaSeconds :type "Float (single-precision)"))
  (set `self.Delta Time` DeltaSeconds)
  (`|ExecutionSequence`
    (:`then_0`
      (if (`self.TrueSkyEnabled`)
        _))
    (:`then_1`
      (`self.UpdatePostProcessingVolumes` false))))

(fn `GetCurrentTime`
  (returns (WorldTime :type "Float (double-precision)"))
  (return (+ (`KismetMathLibrary.Conv_IntToDouble` (`self.CurrentDays`)) (/ (`KismetMathLibrary.Conv_IntToDouble` (`self.CurrentHours`)) 24.0) (/ (/ (`KismetMathLibrary.Conv_IntToDouble` (`self.CurrentMinutes`)) 60.0) 24.0) (/ (/ (/ (`self.CurrentSeconds`) 60.0) 60.0) 24.0) (* (`KismetMathLibrary.Conv_IntToDouble` (`self.CurrentMonths`)) 30.0))))

(fn `UpdatePostProcessingVolumes`
  (params (Construction :type Boolean))
  (bind _currentsettings (`self.CurrentSettings`))
  (bind _currentsettings_2 (`self.CurrentSettings`))
  (bind _nightsettings (`self.NightSettings`))
  (bind _daysettings (`self.DaySettings`))
  (bind _targetintensity (`self.TargetIntensity`))
  (bind _returnvalue (`KismetMathLibrary.FInterpTo` (`self.AmbientCubemapIntensity`) (`self.TargetIntensity`) (`self.Delta Time`) (`self.AmbientCubemapIntensitySpeed`)))
  (bind _returnvalue_2 (`self.Get2400Format`))
  (for _array_element (`self.PostProcessVolumes`)
    (set `self.AmbientCubemapIntensity` (`.AmbientCubemapIntensity` (break `Scene.PostProcessSettings` (`PostProcessVolume.Settings` _array_element))))
    (if Construction
      (bind _returnvalue_3 (or (>= _returnvalue_2 (`self.DayEndTIme`)) (< _returnvalue_2 (`self.DayStartTime`))))
      (if _returnvalue_3
        (set `self.TargetIntensity` (`.AmbientCubemapIntensity` (break `Scene.PostProcessSettings` (`self.NightSettings`))))
        (set `self.CurrentSettings` (`self.NightSettings`))
        (setmembers `Scene.PostProcessSettings` :`StructRef` _currentsettings :`AmbientCubemapIntensity` _targetintensity)
        (set `PostProcessVolume.Settings` _currentsettings _array_element)
        (else
          (set `self.TargetIntensity` (`.AmbientCubemapIntensity` (break `Scene.PostProcessSettings` (`self.DaySettings`))))
          (set `self.CurrentSettings` (`self.DaySettings`))
          (setmembers `Scene.PostProcessSettings` :`StructRef` _currentsettings :`AmbientCubemapIntensity` _targetintensity)
          (set `PostProcessVolume.Settings` _currentsettings _array_element)))
      (elif _returnvalue_3
        (set `self.TargetIntensity` (`.AmbientCubemapIntensity` (break `Scene.PostProcessSettings` _nightsettings)))
        (set `self.CurrentSettings` _nightsettings)
        (setmembers `Scene.PostProcessSettings` :`StructRef` _currentsettings_2 :`AmbientCubemapIntensity` _returnvalue)
        (set `PostProcessVolume.Settings` _currentsettings_2 _array_element)
        (else
          (set `self.TargetIntensity` (`.AmbientCubemapIntensity` (break `Scene.PostProcessSettings` _daysettings)))
          (set `self.CurrentSettings` _daysettings)
          (setmembers `Scene.PostProcessSettings` :`StructRef` _currentsettings_2 :`AmbientCubemapIntensity` _returnvalue)
          (set `PostProcessVolume.Settings` _currentsettings_2 _array_element))))
    (return))
  (return))

(fn `UserConstructionScript`
  (`/Engine/EditorBlueprintResources/StandardMacros.IsValid` (`self.Sun`)
    (:`Is Valid`
      (`/Engine/EditorBlueprintResources/StandardMacros.IsValid` null
        (:`Is Valid`
          (bind _worldtime (`self.GetCurrentTime`)))))))