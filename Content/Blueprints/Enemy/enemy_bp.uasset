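; Enemy actor Blueprint that tracks its own health and reacts to damage.
; AnyDamage spawns a blood particle effect offset from Box1, subtracts the damage from Health and prints the result; Health is clamped only at BeginPlay.
; Tick unhides the player's pawn, not the enemy, whenever Health is at or below a threshold.
; Unconnected nodes for showing or destroying the player character's mesh never run.
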(event `self.ReceiveTick`
  (params (DeltaSeconds :type "Float (single-precision)"))
  (if (<= (`self.Health`) 80.0)
    (`self.SetActorHiddenInGame` (`GameplayStatics.GetPlayerPawn` 0) false)))

(event `self.ReceiveAnyDamage`
  (params (Damage :type "Float (single-precision)") (DamageType :type "DamageType Object Reference") (InstigatedBy :type "Controller Object Reference") (DamageCauser :type "Actor Object Reference"))
  (bind _health (`self.Health`))
  ;[1 1 1] Get Damage
  (`GameplayStatics.SpawnEmitterAtLocation` "/Game/Particles/Character/P_blood.P_blood" (+ (`SceneComponent.K2_GetComponentLocation` (`self.Box1`)) (30.0 -10.0 100.0)))
  (set `self.Health` (- _health Damage))
  (`KismetSystemLibrary.PrintString` (`KismetStringLibrary.Concat_StrStr` "Enemy Health" (`KismetStringLibrary.Conv_DoubleToString` _health))))

(event `self.ReceiveBeginPlay`
  (bind _health (`self.Health`))
  ;[1 1 1] Set Base Health
  (set `self.Health` (`KismetMathLibrary.FClamp` _health 0.0 100.0))
  (`KismetSystemLibrary.PrintString` (`KismetStringLibrary.Concat_StrStr` "Enemy Health" (`KismetStringLibrary.Conv_DoubleToString` _health))))

(fn `UserConstructionScript`)