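; HUD Blueprint for the Caede character that turns mouse motion into scroll input for inventory navigation.
; Tick polls the cursor to fire custom move and move-ended dispatchers, and binds or unbinds inventory handlers as the character's input mode changes.
; The move handler stores the offset from screen center and re-centers the cursor, making it a relative input.
; SelectItem provides wrap-around index cycling but is not called in this Blueprint.
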(event Custom|OnMouseMoveEnded_Even_inventory
  (params (Current :type Vector%202D%20Structure) (Last :type Vector%202D%20Structure))
  ;[1 0.06756 0 0.56] Inventory Navigation Ended
  (Variables|InventoryMode|SetInventoryScrollStarted false)
  (Variables|InventoryMode|SetDeltaInventoryScroll 0)
  (Variables|InventoryModeItemDetails|SetDeltaItemScroll 0))

(event Custom|OnMouseMoved_Event_Inventory
  (params (Current :type Vector%202D%20Structure) (Last :type Vector%202D%20Structure))
  (bind _returnvalue (Game|GetPlayerController 0))
  (bind (_sizex _sizey) (HUD|GetViewportSize _returnvalue))
  (bind _returnvalue_2 (/ _sizex 2))
  (bind _returnvalue_3 (/ _sizey 2))
  (bind _returnvalue_4 (Math|Conversions|ToFloat(Integer) _returnvalue_2))
  (bind _returnvalue_5 (Math|Conversions|ToFloat(Integer) _returnvalue_3))
  (bind _returnvalue_6 (Math|Vector2D|MakeVector2D _returnvalue_4 _returnvalue_5))
  (bind _returnvalue_7 (- _returnvalue_6 Current))
  (bind (_x _y) (Math|Vector2D|BreakVector2D _returnvalue_7))
  ;[0 0.00901 1 0.56] Inventory Navigation Update
  (Variables|Mouse|SetDeltaScrollX _x)
  (Variables|Mouse|SetDeltaScrollY _y)
  (if (Variables|InventoryMode|GetInventoryModeActive)
    (if (Variables|InventoryMode|GetInventoryScrollStarted)
      _
      (else
        (Variables|InventoryMode|SetInventoryScrollStarted true))))
  (CallFunction|CenterMouse))

(event EventTick
  (params (DeltaSeconds :type Float%20%28single-precision%29))
  (bind _returnvalue (Game|GetPlayerController 0))
  (bind (_sizex _sizey) (HUD|GetViewportSize _returnvalue))
  (bind _returnvalue_2 (/ _sizex 2))
  (bind _returnvalue_3 (/ _sizey 2))
  ;[1 0.3776 0 0.646] Event Tick
  (Variables|Default|SetDelta%20Time DeltaSeconds)
  (Utilities|FlowControl|Sequence
    (:then_0
      ;;[1 1 1] Fire the Mouse Moved Event
      (bind (_x _y) (Class|CaedeHUD|GetMousePosition (Game|Player|GetOwningPlayerController)))
      (Variables|Mouse|SetCurrentMousePosition (Math|Vector2D|MakeVector2D (Math|Conversions|ToFloat(Integer) _x) (Math|Conversions|ToFloat(Integer) _y)))
      (if (> (Math|Vector2D|Vector2DLength (- (Variables|Mouse|GetCurrentMousePosition) (Variables|Mouse|GetLastMousePosition))) (Variables|Mouse|GetMouseMovedTolerance))
        (Default|CallOnMouseMoved (Variables|Mouse|GetCurrentMousePosition) (Variables|Mouse|GetLastMousePosition))
        (Variables|Mouse|SetMoveEnded false)
        (elif (Variables|Mouse|GetMoveEnded)
          _
          (else
            (Default|CallOnMouseMoveEnded (Variables|Mouse|GetCurrentMousePosition))
            (Variables|Mouse|SetMoveEnded true))))
      (Variables|Mouse|SetLastMousePosition (Variables|Mouse|GetCurrentMousePosition)))
    (:then_1
      (bind _asbp_caedecharacter_c (Utilities|Casting|CastToBP_CaedeCharacter (Pawn|GetControlledPawn (Game|Player|GetOwningPlayerController))))
      (Variables|Default|SetOwningCharacter _asbp_caedecharacter_c)
      (Utilities|IsValid (Variables|Default|GetOwningCharacter)
        (:Is%20Valid
          (if (Utilities|Enum|Equal(Enum) (Variables|/Script/Caede.CaedeCharacter|GetCurrentInputMode (Variables|Default|GetOwningCharacter)) "Inventory")
            (if (not (Variables|InventoryMode|GetInventoryModeActive))
              (Class|CaedeHUD|SetMousePosition _returnvalue _returnvalue_2 _returnvalue_3)
              (Variables|Mouse|SetScreenCenter (Math|Vector2D|MakeVector2D (Math|Conversions|ToFloat(Integer) _returnvalue_2) (Math|Conversions|ToFloat(Integer) _returnvalue_3)))
              (Variables|InventoryMode|SetInventoryModeActive true)
              (EventDispatchers|BindEventtoOnMouseMoved (delegate Custom|OnMouseMoved_Event_Inventory))
              (EventDispatchers|BindEventtoOnMouseMoveEnded (delegate Custom|OnMouseMoveEnded_Even_inventory)))
            (else
              (Variables|Default|SetbDrawMouseCross false)
              (Variables|InventoryMode|SetInventoryModeActive false)
              (EventDispatchers|UnbindEventfromOnMouseMoved (delegate Custom|OnMouseMoved_Event_Inventory))
              (EventDispatchers|UnbindEventfromOnMouseMoveEnded (delegate Custom|OnMouseMoveEnded_Even_inventory)))))))))

(fn ConstructionScript)

(fn SelectItem
  (params (CurrentSelectedIndex :type Integer) (Scroll%20Up%20Condition :type Boolean) (Scroll%20Down%20Condition :type Boolean))
  (bind _returnvalue (- CurrentSelectedIndex 1))
  (bind _returnvalue_2 (+ CurrentSelectedIndex 1))
  (bind _selecteditemarray (Variables|InventoryModeItemDetails|GetSelectedItemArray))
  (bind _returnvalue_3 (Utilities|Array|Length _selecteditemarray))
  (Variables|InventoryModeItemDetails|SetNewSelectedItemIndex CurrentSelectedIndex)
  (if (> _returnvalue_3 0)
    (if Scroll%20Down%20Condition
      (if (< _returnvalue 0)
        (Variables|InventoryModeItemDetails|SetNewSelectedItemIndex (- _returnvalue_3 1))
        (else
          (Variables|InventoryModeItemDetails|SetNewSelectedItemIndex _returnvalue)))
      (LocalVariables|SetChangedSelection true :!label _label)
      (elif Scroll%20Up%20Condition
        (if (>= _returnvalue_2 _returnvalue_3)
          (Variables|InventoryModeItemDetails|SetNewSelectedItemIndex 0)
          (goto _label)
          (else
            (Variables|InventoryModeItemDetails|SetNewSelectedItemIndex _returnvalue_2)
            (goto _label)))
        (else
          (LocalVariables|SetChangedSelection false :!label _label_2))))
    (else
      (goto _label_2)))
  (return (Variables|InventoryModeItemDetails|GetNewSelectedItemIndex) (LocalVariables|GetChangedSelection)))

(fn CenterMouse
  (bind _returnvalue (Game|GetPlayerController 0))
  (bind (_sizex _sizey) (HUD|GetViewportSize _returnvalue))
  (Class|CaedeHUD|SetMousePosition _returnvalue (/ _sizex 2) (/ _sizey 2))
  (return))