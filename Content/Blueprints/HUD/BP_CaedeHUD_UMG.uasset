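; HUD Blueprint that creates the circular quick inventory and interaction widgets for the player's Caede character.
; Setup runs from Tick until the character reference is valid, then binds to its input mode change event.
; Entering Inventory mode shows the radial widget and hides crosshairs; other modes hide it and restore the center cross.
; Tick also compares mouse positions against a tolerance to broadcast moved and move-ended events, and a helper recenters the cursor.
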(event `OnInputModeChanged__DelegateSignature_Event`
  (params (NewPlayerInputMode :type "CaedeCharacter.EPlayerInputMode Enum" :default "Move"))
  (bind _quickinventorywidget (`self.QuickInventoryWidget`))
  ;[0.4319 0.01674 1] Begin Play
  ;;[1 1 1] Inventory Activated /Deactivated
  (if (`|EnumEquality` NewPlayerInputMode "Inventory")
    (if (not (`self.InventoryModeActive`))
      (set `self.bDrawMouseCross` false)
      (set `self.bDrawCenterCross` false)
      (set `self.InventoryModeActive` true)
      (bind _ascircle_quick_inventory_widget (cast `/Game/UMG/BaseWidgets/CircleQuickInventoryWidget` _quickinventorywidget))
      (`/Game/UMG/BaseWidgets/CircleQuickInventoryWidget.PerformShow` _ascircle_quick_inventory_widget)
      (else
        (set `self.bDrawMouseCross` false :!label _label)
        (set `self.bDrawCenterCross` true)
        (set `self.InventoryModeActive` false)
        (bind _ascircle_quick_inventory_widget_2 (cast `/Game/UMG/BaseWidgets/CircleQuickInventoryWidget` _quickinventorywidget))
        (`/Game/UMG/BaseWidgets/CircleQuickInventoryWidget.PerformHide` _ascircle_quick_inventory_widget_2)))
    (else
      (goto _label))))

(event `InitialSetup`
  ;[0.4319 0.01674 1] Begin Play
  (bind _asbp_caede_character (cast `/Game/Blueprints/MainCharacter/BP_CaedeCharacter` (`GameplayStatics.GetPlayerCharacter` 0)))
  (set `self.OwningCharacter` _asbp_caede_character)
  (add `/Game/Blueprints/MainCharacter/BP_CaedeCharacter.OnInputModeChanged` (`self.OwningCharacter`) (delegate `OnInputModeChanged__DelegateSignature_Event`))
  (bind _returnvalue (`|CreateWidget` "/Game/UMG/BaseWidgets/CircleQuickInventoryWidget.CircleQuickInventoryWidget_C" (`self.GetOwningPlayerController`)))
  (bind _output_get (set `self.QuickInventoryWidget` _returnvalue))
  (`UserWidget.AddToViewport` _output_get)
  (`/Game/UMG/BaseWidgets/CircleQuickInventoryWidget.PerformHide` _returnvalue)
  (`/Game/UMG/BaseWidgets/CircleQuickInventoryWidget.PerformHide` _returnvalue)
  (bind _returnvalue_2 (`|CreateWidget` "/Game/UMG/BaseWidgets/InteractionWidget.InteractionWidget_C" (`GameplayStatics.GetPlayerController` 0)))
  (bind _output_get_2 (set `self.InteractionWidget` _returnvalue_2))
  (`InteractionBaseWidget.InitWidget` _output_get_2 (`self.OwningCharacter`))
  (`UserWidget.AddToViewport` _output_get_2)
  (`Widget.SetVisibility` _output_get_2 "SelfHitTestInvisible"))

(event `self.ReceiveTick`
  (params (DeltaSeconds :type "Float (single-precision)"))
  (bind _currentmouseposition (`self.CurrentMousePosition`))
  (bind _lastmouseposition (`self.LastMousePosition`))
  ;[1 0.3776 0 0.646] Event Tick
  (set `self.Delta Time` DeltaSeconds)
  (`/Engine/EditorBlueprintResources/StandardMacros.IsValid` (`self.OwningCharacter`)
    (:`Is Valid`
      (`|ExecutionSequence`
        (:`then_0`
          ;;[0.1062 0 1] Fire the Mouse Moved /Mouse Move Ended Event
          (bind (_x _y) (`self.GetMousePosition` (`self.GetOwningPlayerController`)))
          (set `self.CurrentMousePosition` (`KismetMathLibrary.MakeVector2D` (`KismetMathLibrary.Conv_IntToDouble` _x) (`KismetMathLibrary.Conv_IntToDouble` _y)))
          (if (> (`KismetMathLibrary.VSize2D` (- (`self.CurrentMousePosition`) (`self.LastMousePosition`))) (`self.MouseMovedTolerance`))
            (`self.OnMouseMoved` _currentmouseposition _lastmouseposition)
            (set `self.MoveEnded` false)
            (elif (not (`self.MoveEnded`))
              (`self.OnMouseMoveEnded` _currentmouseposition _lastmouseposition)
              (set `self.MoveEnded` true)))
          (set `self.LastMousePosition` (`self.CurrentMousePosition`)))))
    (:`Is Not Valid`
      (`self.InitialSetup`))))

(fn `CenterMouse`
  (bind _returnvalue (`GameplayStatics.GetPlayerController` 0))
  (bind (_sizex _sizey) (`PlayerController.GetViewportSize` _returnvalue))
  (`self.SetMousePosition` _returnvalue (/ _sizex 2) (/ _sizey 2))
  (return))

(fn `UserConstructionScript`)