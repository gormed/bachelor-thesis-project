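; BP_DialogPawn is an NPC dialog pawn whose only logic here is a helper that shows or hides debug icons on NPC tasks.
; ToggleDebugTaskIcons switches on the task's type, casts it to the matching task Blueprint, such as idle, patrol or follow, and sets that Blueprint's billboard hidden-in-game state.
; Count and Invalid types are ignored, and the construction script is empty.
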(fn `ToggleDebugTaskIcons`
  (params (Task :type "NPCTask Object Reference") (Hidden :type Boolean))
  (switch `NPCTask.ENPCTaskType` (`NPCTask.TaskType` Task)
    (:`Idle`
      (bind _asbp_idle_task (cast `/Game/Blueprints/NPCs/Daycycle/BP_IdleTask` Task)
        (:`then`
          (`SceneComponent.SetHiddenInGame` (`/Game/Blueprints/NPCs/Daycycle/BP_IdleTask.Billboard1` _asbp_idle_task) Hidden false))
        (:`CastFailed`
          _)))
    (:`Sleep`
      (bind _asbp_sleep_task (cast `/Game/Blueprints/NPCs/Daycycle/BP_SleepTask` Task)
        (:`then`
          (`SceneComponent.SetHiddenInGame` (`/Game/Blueprints/NPCs/Daycycle/BP_SleepTask.Billboard1` _asbp_sleep_task) Hidden false))
        (:`CastFailed`
          _)))
    (:`Wander`
      (bind _asbp_wander_task (cast `/Game/Blueprints/NPCs/Daycycle/BP_WanderTask` Task)
        (:`then`
          (`SceneComponent.SetHiddenInGame` (`/Game/Blueprints/NPCs/Daycycle/BP_WanderTask.Billboard1` _asbp_wander_task) Hidden false))
        (:`CastFailed`
          _)))
    (:`Patrol`
      (bind _asbp_patrol_task (cast `/Game/Blueprints/NPCs/Daycycle/BP_PatrolTask` Task)
        (:`then`
          (`SceneComponent.SetHiddenInGame` (`/Game/Blueprints/NPCs/Daycycle/BP_PatrolTask.Billboard1` _asbp_patrol_task) Hidden false))
        (:`CastFailed`
          _)))
    (:`Collect`
      (bind _asbp_collect_task (cast `/Game/Blueprints/NPCs/Daycycle/BP_CollectTask` Task)
        (:`then`
          (`SceneComponent.SetHiddenInGame` (`/Game/Blueprints/NPCs/Daycycle/BP_CollectTask.Billboard1` _asbp_collect_task) Hidden false))
        (:`CastFailed`
          _)))
    (:`Hobby`
      (bind _asbp_hobby_task (cast `/Game/Blueprints/NPCs/Daycycle/BP_HobbyTask` Task)
        (:`then`
          (`SceneComponent.SetHiddenInGame` (`/Game/Blueprints/NPCs/Daycycle/BP_HobbyTask.Billboard1` _asbp_hobby_task) Hidden false))
        (:`CastFailed`
          _)))
    (:`Work`
      (bind _asbp_work_task (cast `/Game/Blueprints/NPCs/Daycycle/BP_WorkTask` Task)
        (:`then`
          (`SceneComponent.SetHiddenInGame` (`/Game/Blueprints/NPCs/Daycycle/BP_WorkTask.Billboard1` _asbp_work_task) Hidden false))
        (:`CastFailed`
          _)))
    (:`Follow`
      (bind _asbp_follow_task (cast `/Game/Blueprints/NPCs/Daycycle/BP_FollowTask` Task)
        (:`then`
          (`SceneComponent.SetHiddenInGame` (`/Game/Blueprints/NPCs/Daycycle/BP_FollowTask.Billboard1` _asbp_follow_task) Hidden false))
        (:`CastFailed`
          _)))
    (:`Count`
      _)
    (:`Invalid`
      _))
  (return))

(fn `UserConstructionScript`)