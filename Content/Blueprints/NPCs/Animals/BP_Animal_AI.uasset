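; AI controller for animal NPCs that runs their shared behavior tree.
; On BeginPlay it sets up the animal blackboard, saves the pawn's starting position as HomeLocation, then starts AnimalBehaviourTree.
; A helper computes a yaw-only look-at rotation from just ahead of an actor, but the interpolated turn-toward-focal-point logic using it is disconnected, and Tick does nothing.
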(event `self.ReceiveBeginPlay`
  (`self.UseBlackboard` "/Game/Blueprints/NPCs/Animals/AnimalBlackboard.AnimalBlackboard")
  (`BlackboardComponent.SetValueAsVector` (`self.BlackboardComponent`) (`self.HomeLocation`) (`self.K2_GetActorLocation` (`self.K2_GetPawn`)))
  (`self.RunBehaviorTree` (`self.AnimalBehaviourTree`)))

(event `self.ReceiveTick`
  (params (DeltaSeconds :type "Float (single-precision)")))

(fn `GetLookAtRotation`
  (params (Who :type "Actor Object Reference") (LookAt :type "Object.Vector Structure"))
  (returns (Rotation :type "Object.Rotator Structure"))
  (return (`KismetMathLibrary.MakeRot` 0.0 (.yaw (`KismetMathLibrary.FindLookAtRotation` (+ (`self.K2_GetActorLocation` Who) (* (`self.GetActorForwardVector` Who) 10.0)) LookAt)))))

(fn `UserConstructionScript`)