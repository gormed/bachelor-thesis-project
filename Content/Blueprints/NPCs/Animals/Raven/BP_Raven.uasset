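; Raven NPC that fakes flight on Character movement by calling Jump every tick, with JumpZVelocity driven by a sine/cosine wave.
; The CanJump override flips between climbing and descending at the min and max heights, changing the wave's offset and speed.
; Tick steers toward the AI controller's blackboard WanderLocation with smoothed movement input and banks the roll from the change in heading.
; Optional debug lines show target and input.
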(event `self.ReceiveTick`
  (params (DeltaSeconds :type "Float (single-precision)"))
  (bind _returnvalue (`self.K2_GetActorLocation`))
  (bind _returnvalue_2 (`BlackboardComponent.GetValueAsVector` (`AIBlueprintHelperLibrary.GetBlackboard` (`self.CaedeAIController`)) (`self.WanderLocation`)))
  (bind _returnvalue_3 (* (`self.MovementScale`) (`KismetMathLibrary.VSize` (`self.GetVelocity`))))
  (bind _returnvalue_4 (`KismetMathLibrary.MultiplyByPi` (* (`self.Timer`) (* (`self.InternalSpeedModifier`) 2.0))))
  (bind _returnvalue_5 (`KismetMathLibrary.MakeVector` (.x (`KismetMathLibrary.VInterpTo` (`self.GetActorForwardVector`) (`KismetMathLibrary.Normal` (- _returnvalue_2 _returnvalue)) (`self.DeltaSeconds`) (`self.FaceingDamp`))) (.y (`KismetMathLibrary.VInterpTo` (`self.GetActorForwardVector`) (`KismetMathLibrary.Normal` (- _returnvalue_2 _returnvalue)) (`self.DeltaSeconds`) (`self.FaceingDamp`)))))
  (set `self.DeltaSeconds` DeltaSeconds)
  (set `self.Timer` (+ (`self.DeltaSeconds`) (`self.Timer`)))
  (if (`self.RaiseFlying`)
    (set `self.InternalRaiseAmount` (* (`self.FlyRaiseAmount`) 1.0))
    (set `self.InternalSpeedModifier` (* (`self.FlyAnimationSpeed`) 1.0))
    (else
      (set `self.InternalRaiseAmount` (* (`self.FlyRaiseAmount`) -1.0))
      (set `self.InternalSpeedModifier` (* (`self.FlyAnimationSpeed`) 0.33))))
  (set `CharacterMovementComponent.JumpZVelocity` (+ (* (`KismetMathLibrary.Sin` _returnvalue_4) (`self.FlyAnimationHeightVaration`)) (* (`self.FlyAnimationHeightOffset`) (+ (`KismetMathLibrary.Cos` _returnvalue_4) (`self.InternalRaiseAmount`)))) (`self.CharacterMovement`))
  (bind _ascaede_aicontroller (cast `CaedeAIController` (`self.GetController`)))
  (set `self.CaedeAIController` _ascaede_aicontroller)
  (set `self.FlyCurvature` (- (`KismetMathLibrary.DegAtan2` (.y (`self.LastMovementInput`)) (.x (`self.LastMovementInput`))) (`KismetMathLibrary.DegAtan2` (.y _returnvalue_5) (.x _returnvalue_5))))
  (set `self.LastMovementInput` _returnvalue_5)
  (`self.AddMovementInput` _returnvalue_5 _returnvalue_3)
  (`self.Jump`)
  (set `self.LastRotation` (`KismetMathLibrary.MakeRot` (.pitch (`self.K2_GetActorRotation`)) (.yaw (`self.K2_GetActorRotation`)) (.roll (`KismetMathLibrary.RInterpTo` (`KismetMathLibrary.MakeRot` 0.0 0.0 (.roll (`self.LastRotation`))) (`KismetMathLibrary.MakeRot` 0.0 0.0 (.roll (`KismetMathLibrary.RotatorFromAxisAndAngle` (1.0 0.0 0.0) (* (`self.FlyCurvature`) (`self.DriftAngle`))))) (`self.DeltaSeconds`) (`self.RollSpeed`)))))
  (`self.K2_SetActorRelativeRotation` (`self.LastRotation`))
  (if (`self.DebugDraw`)
    (`KismetSystemLibrary.DrawDebugLine` _returnvalue _returnvalue_2 (struct :`R` 1.0 :`G` 0.015037 :`A` 1.0) 0.1 2.0)
    (`KismetSystemLibrary.DrawDebugLine` _returnvalue (+ _returnvalue (* _returnvalue_5 _returnvalue_3)) (struct :`G` 0.122582 :`B` 1.0 :`A` 1.0) 0.1 2.0)))

(fn `CanJumpInternal`
  (returns (ReturnValue :type Boolean))
  (bind _z (.z (`self.K2_GetActorLocation`)))
  (if (> _z (`self.MaxFlyHeight`))
    (set `self.DoJump` true)
    (set `self.RaiseFlying` false)
    (elif (< _z (`self.InternalMinFlyHeight`))
      (set `self.DoJump` true)
      (set `self.RaiseFlying` true)))
  (return (`self.DoJump`)))

(fn `UserConstructionScript`
  (`parent.UserConstructionScript`)
  (set `self.InternalMinFlyHeight` (`self.MinFlyHeight`)))