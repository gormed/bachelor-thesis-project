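; BP_WanderTask is an NPC day-cycle helper that picks random wander destinations and reports arrival.
; RandomWanderLocation samples a radius centered half the wander range ahead of the NPC, then stores and returns the point.
; It also finds a synchronous path for optional debug drawing, using a separately evaluated random point.
; ReachedWanderLocation compares horizontal distance to the stored point against a given threshold, ignoring height.
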(fn `RandomWanderLocation`
  (params (OwningNPC :type "CaedeNPC Object Reference") (AI :type "CaedeAIController Object Reference"))
  (returns (Location :type "Object.Vector Structure"))
  (bind _returnvalue (`self.K2_GetActorLocation` OwningNPC))
  (bind _wanderrange (`self.WanderRange`))
  (bind _returnvalue_2 (`NavigationSystem.GetRandomPointInRadius` (+ _returnvalue (* (`self.GetActorForwardVector` OwningNPC) (* _wanderrange 0.5))) _wanderrange))
  (bind _returnvalue_3 (`NavigationSystem.FindPathToLocationSynchronously` AI _returnvalue _returnvalue_2 AI))
  (`NavigationPath.EnableDebugDrawing` _returnvalue_3 (`self.DrawDebPAth`) (struct :`R` 1.0 :`G` 1.0 :`B` 1.0 :`A` 1.0))
  (set `self.WanderLocaton` _returnvalue_2)
  (return (`self.WanderLocaton`)))

(fn `ReachedWanderLocation`
  (params (NPC :type "CaedeNPC Object Reference") (Distance :type "Float (double-precision)"))
  (returns (Reached :type Boolean))
  (return (< (`KismetMathLibrary.VSize2D` (- (`KismetMathLibrary.MakeVector2D` (.x (`self.K2_GetActorLocation` NPC)) (.y (`self.K2_GetActorLocation` NPC))) (`KismetMathLibrary.MakeVector2D` (.x (`self.WanderLocaton`)) (.y (`self.WanderLocaton`))))) Distance)))

(fn `UserConstructionScript`)