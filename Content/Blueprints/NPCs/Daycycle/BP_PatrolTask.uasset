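; BP_PatrolTask is an NPC daycycle task that holds a looping patrol route and tracks the current patrol point.
; The construction script selects the first entry of PatrolPoints when it is valid.
; ReachedTargetPoint advances the index, wrapping to the start after the last entry.
; An invalid entry leaves the current point unchanged, although the index still advances.
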(fn `ReachedTargetPoint`
  (bind _item (`KismetArrayLibrary.Array_Get` (`self.PatrolPoints`) (`self.CurrentTaskIndex`)))
  (bind _returnvalue (+ (`self.CurrentTaskIndex`) 1))
  (if (> (`KismetArrayLibrary.Array_Length` (`self.PatrolPoints`)) _returnvalue)
    (set `self.CurrentTaskIndex` _returnvalue)
    (else
      (set `self.CurrentTaskIndex` 0)))
  (`/Engine/EditorBlueprintResources/StandardMacros.IsValid` _item
    (:`Is Valid`
      (set `self.CurrentPatrolPoint` _item))))

(fn `UserConstructionScript`
  (bind _item (`KismetArrayLibrary.Array_Get` (`self.PatrolPoints`)))
  (`/Engine/EditorBlueprintResources/StandardMacros.IsValid` _item
    (:`Is Valid`
      (set `self.CurrentPatrolPoint` _item)
      (set `self.CurrentTaskIndex` 0))))