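; BP_IdleTask is an NPC day-cycle task providing idle locations, range checks and turning helpers.
; Idle spots come from IdlePlace, or a random point near the NPC if none is stored.
; Wander points are randomized around either, and widen the range check, which always fails when wandering without IdlePlace.
; Turning interpolates toward a random target that varies pitch and roll, with yaw fixed at zero.
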(fn `IsInIdleLocationRange`
  (params (NPC :type "CaedeNPC Object Reference") (AcceptableDistance :type "Float (double-precision)"))
  (returns (IsInRange :type Boolean))
  (bind _returnvalue (`self.K2_GetActorLocation` NPC))
  (bind _idleplace (`self.IdlePlace`))
  (bind _idleplace_2 (`self.IdlePlace`))
  (if (`self.WanderWhileIdle`)
    (`/Engine/EditorBlueprintResources/StandardMacros.IsValid` _idleplace_2
      (:`Is Valid`
        (set `self.InRange` (< (`KismetMathLibrary.Abs` (`KismetMathLibrary.VSize` (- (`self.K2_GetActorLocation` _idleplace_2) (`self.K2_GetActorLocation` NPC)))) (+ AcceptableDistance (`self.WanderRange`)))))
      (:`Is Not Valid`
        (set `self.InRange` false)))
    (else
      (`/Engine/EditorBlueprintResources/StandardMacros.IsValid` _idleplace
        (:`Is Valid`
          (set `self.InRange` (< (`KismetMathLibrary.Abs` (`KismetMathLibrary.VSize` (- (`self.K2_GetActorLocation` _idleplace) _returnvalue))) AcceptableDistance)))
        (:`Is Not Valid`
          (set `self.InRange` (< (`KismetMathLibrary.Abs` (`KismetMathLibrary.VSize` (- _returnvalue (`self.CurrentIdleLocation`)))) AcceptableDistance))))))
  (return (`self.InRange`)))

(fn `NewRandomTurnRotation`
  (set `self.TargetTurn` (`KismetMathLibrary.MakeRot` (.pitch (`KismetMathLibrary.RandomRotator` true)) 0.0 (.roll (`KismetMathLibrary.RandomRotator` true)))))

(fn `SetIdleLocation`
  (params (NPC :type "CaedeNPC Object Reference"))
  (bind _idleplace (`self.IdlePlace`))
  (`/Engine/EditorBlueprintResources/StandardMacros.IsValid` _idleplace
    (:`Is Valid`
      (set `self.CurrentIdleLocation` (`self.K2_GetActorLocation` _idleplace)))
    (:`Is Not Valid`
      (if (not (> (`KismetMathLibrary.Abs` (`KismetMathLibrary.VSize` (`self.CurrentIdleLocation`))) 0.0))
        (set `self.CurrentIdleLocation` (`NavigationSystem.GetRandomPointInRadius` (`self.K2_GetActorLocation` NPC) (`self.RandomIdleLocationRadius`)))))))

(fn `SetIdleWanderLocation`
  (params (NPC :type "CaedeNPC Object Reference"))
  (bind _idleplace (`self.IdlePlace`))
  (bind _wanderrange (`self.WanderRange`))
  (`/Engine/EditorBlueprintResources/StandardMacros.IsValid` _idleplace
    (:`Is Valid`
      (set `self.CurrentIdleWanderLocation` (`NavigationSystem.GetRandomPointInRadius` (`self.K2_GetActorLocation` _idleplace) _wanderrange)))
    (:`Is Not Valid`
      (set `self.CurrentIdleWanderLocation` (`NavigationSystem.GetRandomPointInRadius` (`self.K2_GetActorLocation` NPC) _wanderrange)))))

(fn `TickIdleTurn`
  (params (NPC :type "CaedeNPC Object Reference") (DeltaTime :type "Float (double-precision)"))
  (returns (NewRotation :type "Object.Rotator Structure"))
  (return (`KismetMathLibrary.RInterpTo` (`self.K2_GetActorRotation` NPC) (`self.TargetTurn`) DeltaTime (`self.TurnSpeed`))))

(fn `UserConstructionScript`)