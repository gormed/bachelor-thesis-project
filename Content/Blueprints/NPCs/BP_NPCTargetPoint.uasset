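; BP_NPCTargetPoint is an NPC target point with a list of acceptable tasks and a cached list of Item actors inside its collection zone.
; The construction script shows a preview sphere at the zone radius when Collect is an acceptable task, and BeginPlay destroys that sphere.
; At runtime, FindCollectableItems rebuilds the list with a sphere overlap query on BeginPlay and at a timed interval through Tick, regardless of task.
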(event `self.ReceiveBeginPlay`
  (`ActorComponent.K2_DestroyComponent` (`self.Sphere`))
  (`self.FindCollectableItems`))

(event `self.ReceiveTick`
  (params (DeltaSeconds :type "Float (single-precision)"))
  (set `self.UpdateTimer` (+ DeltaSeconds (`self.UpdateTimer`)))
  (if (> (`self.UpdateTimer`) (`self.UpdateInterval`))
    (set `self.UpdateTimer` 0.0)
    (`self.FindCollectableItems`)))

(fn `FindCollectableItems`
  (bind _collectableitems (`self.CollectableItems`))
  (`KismetArrayLibrary.Array_Clear` (`self.CollectableItems`))
  (bind (_outactors _returnvalue) (`KismetSystemLibrary.SphereOverlapActors_NEW` (`self.K2_GetActorLocation`) (`self.CollectionZoneRadius`) (`self.CollectableObjectTypes`) "/Script/Caede.Item" (`|MakeArray` self :!type "Actor Object Reference")))
  (if _returnvalue
    (for _array_element _outactors
      (bind _asitem (cast `Item` _array_element))
      (if (not (`KismetArrayLibrary.Array_Contains` _collectableitems _asitem))
        (`KismetArrayLibrary.Array_Add` _collectableitems _asitem)))))

(fn `UserConstructionScript`
  (bind _sphere (`self.Sphere`))
  (`KismetArrayLibrary.Array_Clear` (`self.CollectableItems`))
  (`SceneComponent.SetVisibility` (`self.Sphere`) false false)
  (for _array_element (`self.AcceptableTasks`)
    (if (`|EnumEquality` _array_element "Collect")
      (`SphereComponent.SetSphereRadius` _sphere (`self.CollectionZoneRadius`) false)
      (`SceneComponent.SetVisibility` _sphere true false)
      (`self.FindCollectableItems`)
      (break))))